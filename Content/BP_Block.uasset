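; BP_Block is a breakable block that loses one HP per hit and is destroyed at zero.
; It registers itself with BP_GameManager on BeginPlay and reports when broken, so the manager can count blocks.
; ReloadHp shows the remaining HP on a text render and tints a dynamic material, created in the construction script, using a color table indexed by HP.
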(event EventBeginPlay
  (bind _returnvalue (Actor|GetActorOfClass "/Game/BP_GameManager.BP_GameManager_C"))
  (Default|AddBlockNum _returnvalue)
  (CallFunction|ReloadHp))

(event Collision|EventActorBeginOverlap
  (params (OtherActor :type Actor%20Object%20Reference)))

(event EventTick
  (params (DeltaSeconds :type Float%20%28single-precision%29)))

(event Collision|EventHit
  (params (MyComp :type Primitive%20Component%20Object%20Reference) (Other :type Actor%20Object%20Reference) (OtherComp :type Primitive%20Component%20Object%20Reference) (bSelfMoved :type Boolean) (HitLocation :type Vector :default "0, 0, 0") (HitNormal :type Vector :default "0, 0, 0") (NormalImpulse :type Vector :default "0, 0, 0") (Hit :type Hit%20Result%20Structure%20%28by%20ref%29))
  (Variables|Default|SetHp (- (Variables|Default|GetHp) 1))
  (CallFunction|ReloadHp)
  (if (<= (Variables|Default|GetHp) 0)
    (Actor|DestroyActor)
    (bind _returnvalue (Actor|GetActorOfClass "/Game/BP_GameManager.BP_GameManager_C"))
    (Default|AddBrokenBlockNum _returnvalue)))

(fn ConstructionScript
  (bind _returnvalue (Rendering|Material|CreateDynamicMaterialInstance (Variables|Default|GetCube) 0 "/Game/BlockMaterial.BlockMaterial" "None" :!class /Script/Engine.PrimitiveComponent))
  (Variables|Default|SetMaterialInstance _returnvalue))

(fn ReloadHp
  (bind _hp (Variables|Default|GetHp))
  (bind _returnvalue (- _hp 1))
  (Rendering|Components|TextRender|SetText (Variables|Default|GetTextRender) (Utilities|Text|ToText(Integer) (Variables|Default|GetHp)))
  (if (Utilities|Array|IsValidIndex (Variables|Default|GetColorTable) _returnvalue)
    (Rendering|Material|SetVectorParameterValue (Variables|Default|GetMaterialInstance) "BaseColor" (Utilities|Array|Get(acopy) (Variables|Default|GetColorTable) _returnvalue) :!class /Script/Engine.MaterialInstanceDynamic)))